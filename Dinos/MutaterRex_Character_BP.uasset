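; Mutater Rex dino character that can gain extra random mutations when it levels up, until both lineage counters hit the cap.
; Mutation odds climb exponentially with failed attempts; success adds points to a weighted-random stat, bumps a matrilineal or patrilineal count and may recolor a region.
; Stats and counts reach clients through multicast and RepNotify.
; A team-only multi-use wheel page lists mutations, and INI-gated logging relays client messages to the server.
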(event Custom|MC%20Update%20Stat
  (params (Stat :type EPrimalCharacterStatusValue%20Enum :default "Health") (Max%20Value :type Float%20%28single-precision%29) (Current%20Value :type Float%20%28single-precision%29) (Mat%20Mutations :type Integer) (Pat%20Mutations :type Integer))
  (bind _mycharacterstatuscomponent (Variables|Default|GetMyCharacterStatusComponent))
  ;[1 1 0 0.5] MC Mutated Stat Change Values to Relevant Clients
  (if (not (Networking|IsServer))
    (Variables|Default|SetRandomMutationsFemale Mat%20Mutations)
    (Variables|Default|SetRandomMutationsMale Pat%20Mutations)
    (Class|PrimalCharacterStatusComponent|SetMaxStatusValue _mycharacterstatuscomponent Stat Max%20Value)
    (Class|PrimalCharacterStatusComponent|ModifyCurrentStatusValue _mycharacterstatuscomponent Stat Current%20Value false false false true 0 false false)
    (Class|PrimalCharacterStatusComponent|TickStatus _mycharacterstatuscomponent 0.05 false)))

(event EventBeginPlay
  ;[0 1 0 0.5] Begin Play - Setup Matrilineal/Patrilineal Counts for Clients
  (|CallParentFunction)
  (if (and (Networking|IsServer) (Class|PrimalDinoCharacter|BPIsTamed))
    (Utilities|FlowControl|RetriggerableDelay (Math|Random|RandomFloatinRange 0.4 0.8))
    (Variables|MutationStatsRuntimeTracked|SetREPMutationsFemale (Variables|Default|GetRandomMutationsFemale) true)
    (Variables|MutationStatsRuntimeTracked|SetREPMutationsMale (Variables|Default|GetRandomMutationsMale) true)))

(fn ConstructionScript
  (|CallParentFunction)
  (if (Networking|IsServer)
    (Utilities|Array|AppendArray (Variables|MutationStatsRuntimeTracked|GetExtraMutations) (Utilities|Array|MakeArray 0 0 0 0 0 0 0 0 0 0 0 0))))

(fn BPNotifyLevelUp
  (params (ExtraCharacterLevel :type Integer))
  (bind _mutatecoefficient (Variables|MutationStatsDefaults|GetMutateCoefficient))
  (bind _l_extramutes (LocalVariables|GetL_ExtraMutes))
  (bind _randommutationsfemale (Variables|Default|GetRandomMutationsFemale))
  (bind _randommutationsmale (Variables|Default|GetRandomMutationsMale))
  (bind _maxallowedrandommutations (Variables|Default|GetMaxAllowedRandomMutations))
  (if (or (< _randommutationsfemale _maxallowedrandommutations) (< _randommutationsmale _maxallowedrandommutations))
    (LocalVariables|SetL_Roll (Math|Random|RandomFloatinRange 0.0 1e+02))
    (LocalVariables|SetL_Chance (Math|Float|Clamp(Float) (+ _mutatecoefficient (Math|Float|Power _mutatecoefficient (Math|Conversions|ToFloat(Integer) (Variables|MutationStatsRuntimeTracked|GetMutateAttempts)))) 1.0 99.0))
    (if (<= (LocalVariables|GetL_Roll) (LocalVariables|GetL_Chance))
      (bind _stat (CallFunction|ChooseMutateStat))
      (LocalVariables|SetL_MutateStat _stat)
      (Variables|MutationStatsRuntimeTracked|SetMutateAttempts 0)
      (Utilities|Array|AppendArray _l_extramutes (Variables|MutationStatsRuntimeTracked|GetExtraMutations))
      (Utilities|Array|SetArrayElem _l_extramutes (LocalVariables|GetL_MutateStat) (+ (Utilities|Array|Get(acopy) _l_extramutes (LocalVariables|GetL_MutateStat)) 1))
      (Variables|MutationStatsRuntimeTracked|SetExtraMutations _l_extramutes true)
      (CallFunction|MutateStat (LocalVariables|GetL_MutateStat))
      (LocalVariables|SetL_Roll (Math|Random|RandomFloatinRange 0.0 1e+02))
      (if (<= (LocalVariables|GetL_Roll) (Math|Float|Clamp(Float) (Math|Float|SelectFloat (Variables|MutationStatsDefaults|GetMutateColorChance) (Variables|MutationStatsDefaults|GetMutateColorChancePIE) (Class|VictoryCore|IsShipping)) 0.0 1e+02))
        (LocalVariables|SetL_ColorRegion (Math|Random|RandomIntegerinRange 0 5))
        (bind _colorid (CallFunction|ChooseRandomColor))
        (Class|PrimalDinoCharacter|ForceUpdateColorSets (LocalVariables|GetL_ColorRegion) _colorid)
        (Class|PrimalDinoCharacter|RefreshColorization true)
        (Log|MutaterLog "Mutated Color - Region [{0}] New ColorID [{1}]" (Utilities|String|ToString(Integer) (LocalVariables|GetL_ColorRegion)) (Utilities|String|ToString(Integer) _colorid)))
      (else
        (Utilities|FlowControl|Sequence
          (:then_0
            (Log|MutaterLog "Failed Mutate Roll. Attempts [{0}] Roll [{1}] Chance [{2}]" (Utilities|String|ToString(Integer) (Variables|MutationStatsRuntimeTracked|GetMutateAttempts)) (Utilities|String|ToString(Float) (LocalVariables|GetL_Roll)) (Utilities|String|ToString(Float) (LocalVariables|GetL_Chance))))
          (:then_1
            (Variables|MutationStatsRuntimeTracked|SetMutateAttempts (+ (Variables|MutationStatsRuntimeTracked|GetMutateAttempts) 1))))))
    (else
      (Log|MutaterLog "Mutations are at MAX!!! Mat Muts [{0}] Pat Muts [{1}] Max is [{2}]" (Utilities|String|ToString(Integer) _randommutationsfemale) (Utilities|String|ToString(Integer) _randommutationsmale) (Utilities|String|ToString(Integer) _maxallowedrandommutations)))))

(fn ChooseMutateStat
  (Utilities|FlowControl|Sequence
    (:then_0
      (for (_array_element _array_index) (Variables|MutationStatsDefaults|GetMutateEligibleStatWeights)
        (if (> _array_element 0)
          (LocalVariables|SetL_WgtSum (+ (LocalVariables|GetL_WgtSum) (Math|Conversions|ToInteger(Byte) _array_element)))
          (bind _returnvalue (Utilities|Array|Add (LocalVariables|GetL_Stats) _array_index))
          (Utilities|Array|SetArrayElem (LocalVariables|GetL_Wgts) _returnvalue (Math|Conversions|ToInteger(Byte) _array_element) true))))
    (:then_1
      (LocalVariables|SetL_Roll (Math|Random|RandomIntegerinRange 1 (LocalVariables|GetL_WgtSum)))
      (bind (_array_element_2 _array_index_2) (Utilities|Array|ForEachLoopwithBreak (LocalVariables|GetL_Wgts) :!label _label)
        (:LoopBody
          (if (<= (LocalVariables|GetL_Roll) (+ _array_element_2 (LocalVariables|GetL_RollingBase)))
            (LocalVariables|SetL_Stat (Utilities|Array|Get(acopy) (LocalVariables|GetL_Stats) _array_index_2))
            (goto _label Break)
            (else
              (LocalVariables|SetL_RollingBase (+ _array_element_2 (LocalVariables|GetL_RollingBase))))))))
    (:then_2
      (return (LocalVariables|GetL_Stat)))))

(fn MutateStat
  (params (Stat :type Integer))
  (bind _maxallowedrandommutations (Variables|Default|GetMaxAllowedRandomMutations))
  (bind _mycharacterstatuscomponent (Variables|Default|GetMyCharacterStatusComponent))
  (bind _mycharacterstatuscomponent_2 (Variables|Default|GetMyCharacterStatusComponent))
  (bind _randommutationgivepoints (Variables|Default|GetRandomMutationGivePoints))
  (bind _returnvalue (Math|Float|Floor _randommutationgivepoints))
  (bind _returnvalue_2 (Math|Integer|Max(Integer) _returnvalue 1))
  (LocalVariables|SetL_Stat Stat)
  (Utilities|FlowControl|Sequence
    (:then_0
      (Log|MutaterLog "Mutating Stat [{0}:{1}] ExtraMutsArray [{2}] {3}" (Utilities|String|ToString(Integer) (LocalVariables|GetL_Stat)) (Utilities|String|EnumtoString (Utilities|Enum|ByteToEnumEPrimalCharacterStatusValue (Math|Conversions|ToByte(Integer) (LocalVariables|GetL_Stat)))) (Log|IntArrayDisplay (Variables|MutationStatsRuntimeTracked|GetExtraMutations)) (CallFunction|MutaterFormatString "Mat Muts [{0}] Pat Muts [{1}]" (Utilities|Array|MakeArray (Utilities|String|ToString(Integer) (Variables|Default|GetRandomMutationsFemale)) (Utilities|String|ToString(Integer) (Variables|Default|GetRandomMutationsMale))))))
    (:then_1
      (if (and (< (Variables|Default|GetRandomMutationsFemale) _maxallowedrandommutations) (< (Variables|Default|GetRandomMutationsMale) _maxallowedrandommutations))
        (if (< (Math|Random|RandomFloatinRange 0.0 1e+02) 5e+01)
          (Variables|Default|SetRandomMutationsFemale (+ (Variables|Default|GetRandomMutationsFemale) 1) :!label _label)
          (Variables|MutationStatsRuntimeTracked|SetREPMutationsFemale (Variables|Default|GetRandomMutationsFemale) true)
          (else
            (Variables|Default|SetRandomMutationsMale (+ (Variables|Default|GetRandomMutationsMale) 1) :!label _label_2)
            (Variables|MutationStatsRuntimeTracked|SetREPMutationsMale (Variables|Default|GetRandomMutationsMale) true)))
        (elif (< (Variables|Default|GetRandomMutationsFemale) _maxallowedrandommutations)
          (goto _label)
          (else
            (goto _label_2)))))
    (:then_2
      (Utilities|FlowControl|Sequence
        (:then_0
          (Class|PrimalCharacterStatusComponent|SetLevelUpPoints _mycharacterstatuscomponent_2 (Utilities|Enum|ByteToEnumEPrimalCharacterStatusValue (Math|Conversions|ToByte(Integer) (LocalVariables|GetL_Stat))) false (+ (Class|PrimalCharacterStatusComponent|GetLevelUpPoints _mycharacterstatuscomponent_2 (Utilities|Enum|ByteToEnumEPrimalCharacterStatusValue (Math|Conversions|ToByte(Integer) (LocalVariables|GetL_Stat))) false) _returnvalue_2)))
        (:then_1
          (Class|PrimalCharacterStatusComponent|RescaleMaxStat _mycharacterstatuscomponent_2 (Utilities|Enum|ByteToEnumEPrimalCharacterStatusValue (Math|Conversions|ToByte(Integer) (LocalVariables|GetL_Stat))) 1.0 true))
        (:then_2
          (Class|ActorComponent|SetIsReplicated _mycharacterstatuscomponent_2 true))
        (:then_3
          (Class|PrimalCharacterStatusComponent|SetBaseLevelNoStatChange _mycharacterstatuscomponent_2 (+ (Variables|/Script/ShooterGame.PrimalCharacterStatusComponent|GetBaseCharacterLevel _mycharacterstatuscomponent_2) _returnvalue_2)))
        (:then_4
          (Class|PrimalCharacterStatusComponent|RescaleAllStats _mycharacterstatuscomponent_2))
        (:then_5
          (Class|PrimalCharacterStatusComponent|ServerSyncReplicatedValues _mycharacterstatuscomponent_2))
        (:then_6
          (Class|PrimalCharacterStatusComponent|TickStatus _mycharacterstatuscomponent_2 0.05 false))))
    (:then_3
      (Class|Actor|ForceReplicateNow true false))
    (:then_4
      (CallFunction|MCUpdateStat (Utilities|Enum|ByteToEnumEPrimalCharacterStatusValue (Math|Conversions|ToByte(Integer) (LocalVariables|GetL_Stat))) (Class|PrimalCharacterStatusComponent|BPGetMaxStatusValue _mycharacterstatuscomponent (Utilities|Enum|ByteToEnumEPrimalCharacterStatusValue (Math|Conversions|ToByte(Integer) (LocalVariables|GetL_Stat)))) (Class|PrimalCharacterStatusComponent|BPGetCurrentStatusValue _mycharacterstatuscomponent (Utilities|Enum|ByteToEnumEPrimalCharacterStatusValue (Math|Conversions|ToByte(Integer) (LocalVariables|GetL_Stat)))) (Variables|Default|GetRandomMutationsFemale) (Variables|Default|GetRandomMutationsMale)))))

(fn MutaterFormatString
  (params (Format :type String) (Args :type Array%20of%20Strings))
  (LocalVariables|SetL_Out Format)
  (Utilities|FlowControl|Sequence
    (:then_0
      (for (_array_element _array_index) Args
        (LocalVariables|SetL_Out (Utilities|String|Replace (LocalVariables|GetL_Out) (Utilities|String|Append (Utilities|String|Append "{" (Utilities|String|ToString(Integer) _array_index)) "}") _array_element))))
    (:then_1
      (return (LocalVariables|GetL_Out)))))

(fn MutaterLog
  (params (Log%20Format :type String) (Arg0 :type String) (Arg1 :type String) (Arg2 :type String) (Arg3 :type String))
  (bind _returnvalue (Class|VictoryCore|GetAllLocalPlayerControllers))
  (bind _tamedname (Variables|Default|GetTamedName))
  (bind _item (Utilities|Array|Get(acopy) _returnvalue))
  (if (Log|IsLogEnabled)
    (Utilities|FlowControl|Sequence
      (:then_0
        (LocalVariables|SetL_Log (CallFunction|MutaterFormatString "[{0}] {1}" (Utilities|Array|MakeArray (Utilities|String|SelectString _tamedname (Variables|Default|GetDescriptiveName) (> (Utilities|String|Len _tamedname) 0)) Log%20Format))))
      (:then_1
        (LocalVariables|SetL_Log (CallFunction|MutaterFormatString (LocalVariables|GetL_Log) (Utilities|Array|MakeArray Arg0 Arg1 Arg2 Arg3))))
      (:then_2
        (if (Class|VictoryCore|IsShipping)
          (if (Networking|IsServer)
            (bind _asshootergamemode (Utilities|Casting|CastToShooterGameMode (Game|GetGameMode)))
            (Class|ShooterGameMode|PrinttoServerGameLog _asshootergamemode (LocalVariables|GetL_Log) false)
            (elif (Utilities|Array|IsValidIndex _returnvalue)
              (Utilities|IsValid _item
                (:Is%20Valid
                  (Class|PlayerController|ClientSendNetExecCommandtoServer _item self "Log" (Utilities|Struct|MakeBPNetExecParams 0 0 0 0.0 0.0 0.0 0 0 0 (LocalVariables|GetL_Log)) true)))))
          (else
            (Development|PrintString (LocalVariables|GetL_Log) false)))))))

(fn IsLogEnabled
  (Utilities|FlowControl|Sequence
    (:then_0
      (switch int (Variables|Log|GetLogEnabledSwitch)
        (:0
          (if (Networking|IsServer)
            (bind _asshootergamemode (Utilities|Casting|CastToShooterGameMode (Game|GetGameMode)))
            (bind _returnvalue (Class|ShooterGameMode|GetBoolOptionIni _asshootergamemode "KozDino" "DebugMode" (not (Class|VictoryCore|IsShipping))))
            (LocalVariables|SetbL_Enabled _returnvalue)
            (if (LocalVariables|GetbL_Enabled)
              (Variables|Log|SetLogEnabledSwitch 1 true)
              (else
                (Variables|Log|SetLogEnabledSwitch 2 true)))))
        (:1
          (LocalVariables|SetbL_Enabled true))
        (:2
          (LocalVariables|SetbL_Enabled false))))
    (:then_1
      (return (LocalVariables|GetbL_Enabled)))))

(fn BPServerHandleNetExecCommand
  (params (FromPC :type Player%20Controller%20Object%20Reference) (CommandName :type Name :default "None") (ExecParams :type BP%20Net%20Exec%20Params%20Structure%20%28by%20ref%29))
  (Utilities|FlowControl|Sequence
    (:then_0
      (switch name CommandName
        (:Log
          (if (Log|IsLogEnabled)
            (Utilities|FlowControl|Sequence
              (:then_0
                (bind _asshooterplayercontroller (Utilities|Casting|CastToShooterPlayerController FromPC))
                (bind _returnvalue (Class|ShooterPlayerController|GetPlayerCharacterName _asshooterplayercontroller))
                (LocalVariables|SetL_PName _returnvalue))
              (:then_1
                (bind _asshootergamemode (Utilities|Casting|CastToShooterGameMode (Game|GetGameMode)))
                (Class|ShooterGameMode|PrinttoServerGameLog _asshootergamemode (CallFunction|MutaterFormatString "[CLIENT] [{0}] {1}" (Utilities|Array|MakeArray (LocalVariables|GetL_PName) (.StringParam1 (Utilities|Struct|BreakBPNetExecParams ExecParams)))) false)
                (LocalVariables|SetbL_ReVal true)))))))
    (:then_1
      (return (LocalVariables|GetbL_ReVal)))))

(fn IntArrayDisplay
  (params (Int%20Array :type Array%20of%20Integers))
  (bind _l_items (LocalVariables|GetL_Items))
  (Utilities|FlowControl|Sequence
    (:then_0
      (for _array_element Int%20Array
        (Utilities|Array|Add _l_items (Utilities|String|ToString(Integer) _array_element))))
    (:then_1
      (return (Utilities|String|JoinStringArray _l_items ",")))))

(fn BPGetMultiUseEntries
  (params (ForPC :type Player%20Controller%20Object%20Reference) (MultiUseEntries :type Array%20of%20Multi%20Use%20Entry%20Structures))
  (bind _returnvalue (Math|Conversions|ToColor(LinearColor) "(R=1.000000,G=0.696000,B=0.195000,A=1.000000)"))
  (bind _returnvalue_2 (|CallParentFunction ForPC MultiUseEntries))
  (if (== (Variables|/Script/Engine.Actor|GetTargetingTeam ForPC) (Variables|Default|GetTargetingTeam))
    (Utilities|Array|Add _returnvalue_2 (Utilities|Struct|MakeMultiUseEntry 0 (Utilities|String|ToString(Text) (Utilities|Text|MakeLiteralText "View Extra Mutations")) 7789 -11111 false false false false false false false false true true false false false false 0 "(B=175,G=175,R=175,A=255)" _returnvalue))
    (Utilities|Array|Add _returnvalue_2 (Utilities|Struct|MakeMultiUseEntry 0 (Utilities|String|ToString(Text) (Utilities|Text|MakeLiteralText "Back [Viewing Extra Mutations]")) 7790 -11111 false false false false false false false false true true false false false false 2 "(B=175,G=175,R=175,A=255)" _returnvalue))
    (CallFunction|AddExtraMutationMUs _returnvalue_2))
  (return _returnvalue_2))

(fn BPClientDoMultiUse
  (params (ForPC :type Player%20Controller%20Object%20Reference) (ClientUseIndex :type Integer))
  (bind _asshooterplayercontroller (Utilities|Casting|CastToShooterPlayerController ForPC))
  (switch int ClientUseIndex
    (:7789
      (Class|ShooterPlayerController|SetMultiUseWheelCategory _asshooterplayercontroller 2))
    (:7790
      (Class|ShooterPlayerController|SetMultiUseWheelCategory _asshooterplayercontroller 0))))

(fn AddExtraMutationMUs
  (params (MUs :type Array%20of%20Multi%20Use%20Entry%20Structures))
  (bind _extramutations (Variables|MutationStatsRuntimeTracked|GetExtraMutations))
  (bind _randommutationsfemale (Variables|Default|GetRandomMutationsFemale))
  (bind _randommutationsmale (Variables|Default|GetRandomMutationsMale))
  (for (_array_element _array_index) (Variables|MutationStatsDefaults|GetMutateEligibleStatWeights)
    (LocalVariables|SetL_TmpCnt 0)
    (if (> _array_element 0)
      (if (Utilities|Array|IsValidIndex _extramutations _array_index)
        (LocalVariables|SetL_TmpCnt (Utilities|Array|Get(acopy) _extramutations _array_index)))
      (Utilities|Array|Add MUs (Utilities|Struct|MakeMultiUseEntry 0 (Utilities|String|ToString(Text) (Utilities|Text|ToText(String) (CallFunction|MutaterFormatString "[{1}] {0}" (Utilities|Array|MakeArray (Utilities|String|EnumtoString (Utilities|Enum|ByteToEnumEPrimalCharacterStatusValue (Math|Conversions|ToByte(Integer) _array_index))) (CallFunction|PadZeroLeft (LocalVariables|GetL_TmpCnt) 2))))) (+ _array_index 7891) (- 20 _array_index) false false false false false false false false true true false false true false 2 "(B=175,G=175,R=175,A=255)" (Math|Conversions|ToColor(LinearColor) (Math|Color|SelectColor "(R=1.000000,G=0.796000,B=0.295000,A=1.000000)" "(R=0.550000,G=0.550000,B=0.550000,A=1.000000)" (> (LocalVariables|GetL_TmpCnt) 0)))))))
  (Utilities|Array|Add MUs (Utilities|Struct|MakeMultiUseEntry 0 (Utilities|String|ToString(Text) (Utilities|Text|ToText(String) (CallFunction|MutaterFormatString "[{0}] Matrilineal Mutations" (Utilities|Array|MakeArray (CallFunction|PadZeroLeft _randommutationsfemale 2))))) 8890 -11 false false false false false false false false true true false false true false 2 "(B=175,G=175,R=175,A=255)" (Math|Conversions|ToColor(LinearColor) (Math|Color|SelectColor "(R=1.000000,G=0.796000,B=0.295000,A=1.000000)" "(R=0.550000,G=0.550000,B=0.550000,A=1.000000)" (> _randommutationsfemale 0)))))
  (Utilities|Array|Add MUs (Utilities|Struct|MakeMultiUseEntry 0 (Utilities|String|ToString(Text) (Utilities|Text|ToText(String) (CallFunction|MutaterFormatString "[{0}] Patrilineal Mutations" (Utilities|Array|MakeArray (CallFunction|PadZeroLeft _randommutationsmale 2))))) 8891 -12 false false false false false false false false true true false false true false 2 "(B=175,G=175,R=175,A=255)" (Math|Conversions|ToColor(LinearColor) (Math|Color|SelectColor "(R=1.000000,G=0.796000,B=0.295000,A=1.000000)" "(R=0.550000,G=0.550000,B=0.550000,A=1.000000)" (> _randommutationsmale 0))))))

(fn PadZeroLeft
  (params (Int :type Integer) (Desired%20Length :type Integer))
  (LocalVariables|SetL_Out (Utilities|String|ToString(Integer) Int))
  (while (< (Utilities|String|Len (LocalVariables|GetL_Out)) (Math|Integer|Max(Integer) Desired%20Length))
    (LocalVariables|SetL_Out (Utilities|String|Append (Utilities|String|MakeLiteralString "0") (LocalVariables|GetL_Out))))
  (return (LocalVariables|GetL_Out)))

(fn OnRepREPMutationsFemale
  (if (not (Networking|IsServer))
    (Variables|Default|SetRandomMutationsFemale (Variables|MutationStatsRuntimeTracked|GetREPMutationsFemale))))

(fn OnRepREPMutationsMale
  (if (not (Networking|IsServer))
    (Variables|Default|SetRandomMutationsMale (Variables|MutationStatsRuntimeTracked|GetREPMutationsMale))))

(fn ChooseRandomColor
  (bind _l_allcolorids (LocalVariables|GetL_AllColorIDs))
  (Utilities|FlowControl|Sequence
    (:then_0
      (bind _returnvalue (Class|PrimalGameData|BPGetGameData))
      (for (_array_element _array_index) (Variables|/Script/ShooterGame.PrimalGameData|GetColorDefinitions _returnvalue)
        (if (and (Utilities|Name|NotEqual(Name) (.ColorName (Utilities|Struct|BreakColorDefinition _array_element)) "None") (> (Utilities|String|Len (Utilities|String|ToString(Name) (.ColorName (Utilities|Struct|BreakColorDefinition _array_element)))) 0))
          (Utilities|Array|Add (LocalVariables|GetL_AllColorIDs) (+ _array_index 1)))))
    (:then_1
      (for (_array_element_2 _array_index_2) (Variables|/Script/ShooterGame.PrimalGameData|GetMasterItemList _returnvalue)
        (if (!= _array_element_2 0)
          (if (Utilities|ClassIsChildOf _array_element_2 "/Game/PrimalEarth/CoreBlueprints/Items/PrimalItemDyeGeneric.PrimalItemDyeGeneric_C")
            (bind _returnvalue_2 (Class|PrimalItem|StaticGetDinoColorSetIndexforItemColorID (Class|PrimalItem|GetItemColorIDfromDyeItemID _array_index_2)))
            (if (> _returnvalue_2 0)
              (Utilities|Array|AddUnique (LocalVariables|GetL_AllColorIDs) _returnvalue_2))))))
    (:then_2
      (if (> (Utilities|Array|Length _l_allcolorids) 0)
        (LocalVariables|SetL_Idx (Math|Random|RandomIntegerinRange 0 (Utilities|Array|LastIndex _l_allcolorids)))
        (LocalVariables|SetL_ColorID (Utilities|Array|Get(acopy) (LocalVariables|GetL_AllColorIDs) (LocalVariables|GetL_Idx)))
        (else
          (LocalVariables|SetL_ColorID 0))))
    (:then_3
      (return (LocalVariables|GetL_ColorID)))))