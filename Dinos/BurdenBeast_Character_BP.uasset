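; Burden Beast dino character that earns a focus point per level-up, spent to cut the carried weight of chosen resource classes.
; A radial-wheel submenu lists each focus, and the server records purchases, then multicasts a delayed re-apply.
; Applying rebuilds inventory item-class weight multipliers and tints the mesh emissive RGB by the first three focus levels.
; On load, unstasis or BeginPlay, the server proportionally caps points to the extra character level.
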(event Custom|MC%20Delay%20Apply%20Resource%20Levels
  (Utilities|Time|SetTimerbyFunctionName self "Apply Resource Focus Levels" (Math|Float|SelectFloat 0.1 4.0 (Networking|IsServer))))

(event Custom|PlayLevelUpAnim
  (Class|PrimalCharacter|PlayAnimEx "/Game/PrimalEarth/Dinos/Trike/Animations/Trike-Cuddle_Montage.Trike-Cuddle_Montage" 1.0 "None" false false false false false 0.0 0.0))

(event EventBPUnstasis
  (|CallParentFunction)
  (Utilities|FlowControl|Sequence
    (:then_0
      (if (Networking|IsServer)
        (CallFunction|CapResourceFocusLevels)))
    (:then_1
      (Utilities|Time|SetTimerbyFunctionName self "Apply Resource Focus Levels" (Math|Float|SelectFloat 0.1 4.0 (Networking|IsServer))))))

(event EventBPPostLoadedfromSaveGame
  (|CallParentFunction)
  (Utilities|FlowControl|Sequence
    (:then_0
      (if (Networking|IsServer)
        (CallFunction|CapResourceFocusLevels)))
    (:then_1
      (Utilities|Time|SetTimerbyFunctionName self "Apply Resource Focus Levels" (Math|Float|SelectFloat 0.1 4.0 (Networking|IsServer))))))

(event EventBeginPlay
  (|CallParentFunction)
  (Utilities|FlowControl|Sequence
    (:then_0
      (if (Networking|IsServer)
        (CallFunction|CapResourceFocusLevels)))
    (:then_1
      (Utilities|Time|SetTimerbyFunctionName self "Apply Resource Focus Levels" (Math|Float|SelectFloat 0.1 4.0 (Networking|IsServer))))))

(event EventBPResetClone
  (bind _resourcefocuslevels (Variables|BurdenBeastResourceFocus|GetResourceFocusLevels))
  (for (_ _array_index) _resourcefocuslevels
    (Utilities|Array|SetArrayElem _resourcefocuslevels _array_index 0)
    (Variables|BurdenBeastResourceFocus|SetBurdenBeastLevelUpsAvailable 0 false)))

(fn ConstructionScript
  (bind _resourcefocuslevels (Variables|BurdenBeastResourceFocus|GetResourceFocusLevels))
  (|CallParentFunction)
  (Utilities|Array|Clear _resourcefocuslevels)
  (for _array_element (Variables|BurdenBeastResourceFocus|GetResourceFocusStrings)
    (Utilities|Array|Add _resourcefocuslevels 0)))

(fn CapResourceFocusLevels
  (bind _mycharacterstatuscomponent (Variables|Default|GetMyCharacterStatusComponent))
  (bind _returnvalue (Class|PrimalCharacterStatusComponent|GetExtraCharacterLevel _mycharacterstatuscomponent))
  (LocalVariables|SetL_TotalRF (Math|Conversions|ToFloat(Integer) (Variables|BurdenBeastResourceFocus|GetBurdenBeastLevelUpsAvailable)))
  (for _array_element (Variables|BurdenBeastResourceFocus|GetResourceFocusLevels)
    (LocalVariables|SetL_TotalRF (+ (LocalVariables|GetL_TotalRF) (Math|Conversions|ToFloat(Integer) _array_element))))
  (if (> (LocalVariables|GetL_TotalRF) (Math|Conversions|ToFloat(Integer) _returnvalue))
    (LocalVariables|SetL_RemainingRF _returnvalue)
    (for (_array_element_2 _array_index) (Variables|BurdenBeastResourceFocus|GetResourceFocusLevels)
      (LocalVariables|SetL_NewVal (Math|Integer|Min(Integer) (Math|Float|Floor (* (Math|Conversions|ToFloat(Integer) _returnvalue) (/ (Math|Conversions|ToFloat(Integer) _array_element_2) (LocalVariables|GetL_TotalRF)))) (LocalVariables|GetL_RemainingRF)))
      (LocalVariables|SetL_RemainingRF (- (LocalVariables|GetL_RemainingRF) (LocalVariables|GetL_NewVal)))
      (Utilities|Array|SetArrayElem (Variables|BurdenBeastResourceFocus|GetResourceFocusLevels) _array_index (LocalVariables|GetL_NewVal)))
    (Variables|BurdenBeastResourceFocus|SetBurdenBeastLevelUpsAvailable (LocalVariables|GetL_RemainingRF) false)))

(fn AddLevelUpEntries
  (params (MU%20Entries :type Array%20of%20Multi%20Use%20Entry%20Structures))
  (bind _maxmucolorchannel (Variables|Default|GetMaxMUColorChannel))
  (bind _resourcefocuslevels (Variables|BurdenBeastResourceFocus|GetResourceFocusLevels))
  (bind _minmucolorchannel (Variables|Default|GetMinMUColorChannel))
  (bind _returnvalue (Utilities|Array|Length _resourcefocuslevels))
  (for (_ _array_index) _resourcefocuslevels
    (Utilities|Array|Add MU%20Entries (Utilities|Struct|MakeMultiUseEntry 0 (CallFunction|MakeUseEntryString _array_index) (+ _array_index 27770) (+ _array_index (- _returnvalue _array_index) -5 (* _returnvalue -1)) false (not (or (> (Variables|BurdenBeastResourceFocus|GetBurdenBeastLevelUpsAvailable) 0) (Variables|Default|GetbTestTheBeastOfBurden))) false false false false false false true true false false true false 2 (Math|Color|MakeColor 200 200 200 200) (Math|Conversions|ToColor(LinearColor) (Utilities|Struct|MakeLinearColor (Math|Float|Clamp(Float) (.R (Utilities|Struct|BreakLinearColor (Utilities|Array|Get(acopy) (Variables|BurdenBeastResourceFocus|GetResourceFocusColors) _array_index))) _minmucolorchannel _maxmucolorchannel) (Math|Float|Clamp(Float) (.G (Utilities|Struct|BreakLinearColor (Utilities|Array|Get(acopy) (Variables|BurdenBeastResourceFocus|GetResourceFocusColors) _array_index))) _minmucolorchannel _maxmucolorchannel) (Math|Float|Clamp(Float) (.B (Utilities|Struct|BreakLinearColor (Utilities|Array|Get(acopy) (Variables|BurdenBeastResourceFocus|GetResourceFocusColors) _array_index))) _minmucolorchannel _maxmucolorchannel) 1.0))))))

(fn MakeUseEntryString
  (params (Index :type Integer))
  (bind _resourcefocuslevels (Variables|BurdenBeastResourceFocus|GetResourceFocusLevels))
  (bind _item (Utilities|Array|Get(acopy) _resourcefocuslevels Index))
  (LocalVariables|SetL_RetVal (Utilities|String|Append (Utilities|String|Append (Utilities|String|Append (Utilities|String|SelectString "+Reduce Burden " "Reduce Burden " (> 0 0)) (Utilities|String|Append (Utilities|Array|Get(acopy) (Variables|BurdenBeastResourceFocus|GetResourceFocusStrings) Index) ":  ")) (Utilities|String|Append (Utilities|String|ToString(Text) (Utilities|Text|ToText(Float) (* (- 1.0 (* _item (Utilities|Array|Get(acopy) (Variables|BurdenBeastResourceFocus|GetResourceFocusValuesPerLevel) Index))) 1e+02) "HalfToEven" true 1 324 0 1)) "%")) (Utilities|String|Append " [" (Utilities|String|Append (Utilities|String|ToString(Integer) _item) "]"))))
  (return (LocalVariables|GetL_RetVal)))

(fn ResourceFocusLevelUp
  (params (Use%20Index :type Integer))
  (bind _returnvalue (- Use%20Index 27770))
  (bind _resourcefocuslevels (Variables|BurdenBeastResourceFocus|GetResourceFocusLevels))
  (if (and (Networking|IsServer) (or (> (Variables|BurdenBeastResourceFocus|GetBurdenBeastLevelUpsAvailable) 0) (Variables|Default|GetbTestTheBeastOfBurden)))
    (Variables|BurdenBeastResourceFocus|SetBurdenBeastLevelUpsAvailable (Math|Integer|Max(Integer) 0 (- (Variables|BurdenBeastResourceFocus|GetBurdenBeastLevelUpsAvailable) 1)) false)
    (Utilities|Array|SetArrayElem _resourcefocuslevels _returnvalue (+ (Utilities|Array|Get(acopy) _resourcefocuslevels _returnvalue) 1)))
  (Utilities|FlowControl|Sequence
    (:then_0
      (if (Networking|IsServer)
        (CallFunction|MCDelayApplyResourceLevels)))
    (:then_1
      (if (Class|VictoryCore|IsTimeSince (Class|Actor|GetWorld) (Variables|BurdenBeastResourceFocus|GetLastLevelUpTime) 2.0 true)
        (CallFunction|PlayLevelUpAnim)
        (Variables|BurdenBeastResourceFocus|SetLastLevelUpTime (Utilities|Time|GetGameTimeinSeconds))))))

(fn GetCurrentResourceFocusLevel
  (LocalVariables|SetL_RetVal 0)
  (for _array_element (Variables|BurdenBeastResourceFocus|GetResourceFocusLevels)
    (LocalVariables|SetL_RetVal (+ (LocalVariables|GetL_RetVal) _array_element)))
  (return (LocalVariables|GetL_RetVal)))

(fn BPGetMultiUseEntries
  (params (ForPC :type Player%20Controller%20Object%20Reference) (MultiUseEntries :type Array%20of%20Multi%20Use%20Entry%20Structures))
  (bind _returnvalue (Math|Conversions|ToColor(LinearColor) "(R=1.000000,G=0.696103,B=0.195000,A=1.000000)"))
  (bind _burdenbeastlevelupsavailable (Variables|BurdenBeastResourceFocus|GetBurdenBeastLevelUpsAvailable))
  (bind _returnvalue_2 (Utilities|Text|ToText(Integer) _burdenbeastlevelupsavailable))
  (bind _returnvalue_3 (> _burdenbeastlevelupsavailable 0))
  (bind _returnvalue_4 (Math|Conversions|ToInteger(Boolean) _returnvalue_3))
  (bind _result (Utilities|Text|FormatText "+{NumLevels} Available!" _returnvalue_2))
  (bind _returnvalue_5 (Utilities|String|ToString(Text) _result))
  (bind _returnvalue_6 (Utilities|Select :Index _returnvalue_4 :Option%200 "" :Option%201 _returnvalue_5))
  (if (and (== (Variables|/Script/Engine.Actor|GetTargetingTeam ForPC) (Variables|Default|GetTargetingTeam)) (not (Variables|Default|GetbIsDead)))
    (Utilities|Casting|CastToShooterPlayerController ForPC
      (:then
        (Utilities|Array|Add MultiUseEntries (Utilities|Struct|MakeMultiUseEntry 0 (Utilities|String|Append "View Burden Focus Levels      " _returnvalue_6) 7789 -11111 false false false false false false false false true true false false false false 0 "(B=175,G=175,R=175,A=255)" _returnvalue))
        (Utilities|Array|Add MultiUseEntries (Utilities|Struct|MakeMultiUseEntry 0 (Utilities|String|Append "Back      " _returnvalue_6) 7790 -11111 false false false false false false false false true true false false false false 2 "(B=175,G=175,R=175,A=255)" _returnvalue))
        (CallFunction|AddLevelUpEntries MultiUseEntries))
      (:CastFailed
        _)))
  (return MultiUseEntries))

(fn BPNotifyLevelUp
  (params (ExtraCharacterLevel :type Integer))
  (if (Networking|IsServer)
    (Variables|BurdenBeastResourceFocus|SetBurdenBeastLevelUpsAvailable (+ (Variables|BurdenBeastResourceFocus|GetBurdenBeastLevelUpsAvailable) 1) false)))

(fn BPClientDoMultiUse
  (params (ForPC :type Player%20Controller%20Object%20Reference) (ClientUseIndex :type Integer))
  (bind _asshooterplayercontroller (Utilities|Casting|CastToShooterPlayerController ForPC))
  (switch int ClientUseIndex
    (:7789
      (Class|ShooterPlayerController|SetMultiUseWheelCategory _asshooterplayercontroller 2))
    (:7790
      (Class|ShooterPlayerController|SetMultiUseWheelCategory _asshooterplayercontroller 0))))

(fn BPTryMultiUse
  (params (ForPC :type Player%20Controller%20Object%20Reference) (UseIndex :type Integer))
  (bind _returnvalue (Class|KismetSystemLibrary|MakeLiteralInteger 27770))
  (if (and (>= UseIndex _returnvalue) (< UseIndex (+ _returnvalue (Utilities|Array|Length (Variables|BurdenBeastResourceFocus|GetResourceFocusStrings)))))
    (if (Networking|IsServer)
      (CallFunction|ResourceFocusLevelUp UseIndex)
      (return true))
    (else
      (return true))))

(fn ApplyResourceFocusLevels
  (Utilities|FlowControl|Sequence
    (:then_0
      (for (_array_element _array_index) (Variables|BurdenBeastResourceFocus|GetResourceFocusLevels)
        (Utilities|FlowControl|Sequence
          (:then_0
            (switch int _array_index
              (:0
                (LocalVariables|SetL_G (Math|Float|Max(Float) 0.025 (Math|Float|SelectFloat (Math|Float|Lerp 0.06875 5.0 (Math|Float|Clamp(Float) (* (* (Math|Conversions|ToFloat(Integer) _array_element) (Utilities|Array|Get(acopy) (Variables|BurdenBeastResourceFocus|GetResourceFocusValuesPerLevel) _array_index)) 1.25))) 0.0 (> (* (* (Math|Conversions|ToFloat(Integer) _array_element) (Utilities|Array|Get(acopy) (Variables|BurdenBeastResourceFocus|GetResourceFocusValuesPerLevel) _array_index)) 1.25) 0.0)))))
              (:1
                (LocalVariables|SetL_B (Math|Float|Max(Float) 0.025 (Math|Float|SelectFloat (Math|Float|Lerp 0.06875 5.0 (Math|Float|Clamp(Float) (* (* (Math|Conversions|ToFloat(Integer) _array_element) (Utilities|Array|Get(acopy) (Variables|BurdenBeastResourceFocus|GetResourceFocusValuesPerLevel) _array_index)) 1.25))) 0.0 (> (* (* (Math|Conversions|ToFloat(Integer) _array_element) (Utilities|Array|Get(acopy) (Variables|BurdenBeastResourceFocus|GetResourceFocusValuesPerLevel) _array_index)) 1.25) 0.0)))))
              (:2
                (LocalVariables|SetL_R (Math|Float|Max(Float) 0.025 (Math|Float|SelectFloat (Math|Float|Lerp 0.06875 5.0 (Math|Float|Clamp(Float) (* (* (Math|Conversions|ToFloat(Integer) _array_element) (Utilities|Array|Get(acopy) (Variables|BurdenBeastResourceFocus|GetResourceFocusValuesPerLevel) _array_index)) 1.25))) 0.0 (> (* (* (Math|Conversions|ToFloat(Integer) _array_element) (Utilities|Array|Get(acopy) (Variables|BurdenBeastResourceFocus|GetResourceFocusValuesPerLevel) _array_index)) 1.25) 0.0)))))))
          (:then_1
            (Utilities|Array|AppendArray (LocalVariables|GetL_TotalItemMultipliers) (CallFunction|CreateItemMultiplierArray (Math|Float|Max(Float) (- 1.0 (* (Math|Conversions|ToFloat(Integer) _array_element) (Utilities|Array|Get(acopy) (Variables|BurdenBeastResourceFocus|GetResourceFocusValuesPerLevel) _array_index))) 0.01) (.ClassAdditions (Utilities|Struct|BreakClassAddition (Utilities|Array|Get(acopy) (Variables|BurdenBeastResourceFocus|GetResourceFocusClasses) _array_index)))))))))
    (:then_1
      (Variables|/Script/ShooterGame.PrimalInventoryComponent|SetItemClassWeightMultipliers (Variables|Default|GetMyInventoryComponent) (LocalVariables|GetL_TotalItemMultipliers)))
    (:then_2
      (if (not (Networking|IsDedicatedServer))
        (bind _returnvalue (Rendering|Material|CreateDynamicMaterialInstance (Variables|Character|GetMesh) 0 0 :!class /Script/Engine.PrimitiveComponent))
        (Utilities|IsValid _returnvalue
          (:Is%20Valid
            (Utilities|FlowControl|Sequence
              (:then_0
                (Rendering|Material|SetVectorParameterValue _returnvalue "Emissive - Color and Intensity" (Utilities|Struct|MakeLinearColor (LocalVariables|GetL_R) (LocalVariables|GetL_G) (LocalVariables|GetL_B) 3e+02) :!class /Script/Engine.MaterialInstanceDynamic))
              (:then_1
                (Development|PrintString (Utilities|String|Append (Utilities|String|Append (Utilities|String|Append (Utilities|String|Append "APPLIED COLOR => [" (Utilities|GetDisplayName _returnvalue)) "] VAL [") (Utilities|String|ToString(Integer) (Utilities|Struct|MakeLinearColor (LocalVariables|GetL_R) (LocalVariables|GetL_G) (LocalVariables|GetL_B) 3e+02))) "]") false)))))))))

(fn CreateItemMultiplierArray
  (params (Multipler :type Float%20%28single-precision%29) (Classes :type Array%20of%20Object%20Class%20References))
  (bind _l_itemmultipliers (LocalVariables|GetL_ItemMultipliers))
  (Utilities|FlowControl|Sequence
    (:then_0
      (for _array_element Classes
        (bind _asprimalitem (Utilities|Casting|CastToPrimalItemClass _array_element))
        (Utilities|Array|Add _l_itemmultipliers (Utilities|Struct|MakeItemMultiplier _asprimalitem Multipler))))
    (:then_1
      (return _l_itemmultipliers))))